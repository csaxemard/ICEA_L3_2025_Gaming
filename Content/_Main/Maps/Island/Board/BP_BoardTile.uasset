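; BP_BoardTile is a single board tile actor with a colored cube and a widget that displays its tile ID.
; The construction script gives the cube a dynamic M_TileColor material set to TileColor.
; BeginPlay caches the WBP_TileId widget and disables its shadow, letting SetTileIdAndUpdateWidget update the label.
; A helper returns the cube's scaled dimensions from its bounds; SetTileColor has an empty body.
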(event EventBeginPlay
  (bind _aswbp_tile_id (Utilities|Casting|CastToWBP_TileId (UserInterface|GetUserWidgetObject (Variables|Default|GetWBP_TileId)))
    (:then
      (Variables|Default|SetWBP_TileId-Ref _aswbp_tile_id)
      (Rendering|SetCastShadow (Variables|Default|GetWBP_TileId) false))
    (:CastFailed
      (Development|PrintString "Cast failed"))))

(fn ConstructionScript
  (bind _cube (Variables|Default|GetCube))
  (bind _returnvalue (Rendering|Material|CreateDynamicMaterialInstance _cube 0 "/Game/OldProject/Materials/M_TileColor.M_TileColor" "None" :!class /Script/Engine.PrimitiveComponent))
  (bind _output_get (Variables|Default|SetDynamicMatInstance _returnvalue))
  (Rendering|Material|SetMaterial _cube 0 _output_get)
  (Rendering|Material|SetVectorParameterValue (Variables|Default|GetDynamicMatInstance) "Color" (Variables|Data|GetTileColor) :!class /Script/Engine.MaterialInstanceDynamic))

(fn GetTileScaledDimensions
  (bind _cube (Variables|Default|GetCube))
  (bind (_min _max) (Components|StaticMesh|GetLocalBounds _cube))
  (return (* (Transformation|GetWorldScale _cube) (+ (Math|Vector|VectorGetAbs _min) _max))))

(fn SetTileColor
  (params (TileColor :type Linear%20Color%20Structure)))

(fn SetTileIdandUpdateWidget
  (params (TileId :type Integer))
  (bind _output_get (Variables|Data|SetTileId TileId))
  (Variables|/Script/UMG.TextBlock|SetText (Variables|/Game/_Main/Maps/Island/Board/WBP_TileId.WBP_TileId_C|GetTileId (Variables|Default|GetWBP_TileId-Ref)) (Utilities|Text|ToText(Integer) _output_get)))