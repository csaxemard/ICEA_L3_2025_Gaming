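; Instruction totem on the island map that shows the player a sequence of texts in a WBP_TextBubble widget.
; BeginPlay formats the texts; while the totem is visible, player capsule overlap shows or hides the bubble until all are seen.
; OnInteract advances pages, hides the indicator on the last, then closes, and a later interact replays.
; UnHideTotem reveals the mesh and enables interaction; its overlap re-check is disabled.
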(event OnComponentBeginOverlap(DetectPlayer-SphereCollision)
  (params (OverlappedComponent :type Primitive%20Component%20Object%20Reference) (OtherActor :type Actor%20Object%20Reference) (OtherComp :type Primitive%20Component%20Object%20Reference) (OtherBodyIndex :type Integer) (bFromSweep :type Boolean) (SweepResult :type Hit%20Result%20Structure%20%28by%20ref%29))
  ;[0.15 0.15 0.15 0.5] DetectPlayer
  (if (and (Variables|Default|GetHasSomethingToSay) (Variables|Default|GetisVisible))
    (Utilities|Casting|CastToBP_Player OtherActor)
    (if (Components|ComponentHasTag OtherComp "PlayerMeshCapsule")
      (if (not (Variables|Default|GetallTextSeen))
        (Rendering|SetVisibility (Variables|Default|GetWBP_TextBubble) true false)))))

(event OnComponentEndOverlap(DetectPlayer-SphereCollision)
  (params (OverlappedComponent :type Primitive%20Component%20Object%20Reference) (OtherActor :type Actor%20Object%20Reference) (OtherComp :type Primitive%20Component%20Object%20Reference) (OtherBodyIndex :type Integer))
  ;[0.15 0.15 0.15 0.5] DetectPlayer
  (if (and (Variables|Default|GetHasSomethingToSay) (Variables|Default|GetisVisible))
    (Utilities|Casting|CastToBP_Player OtherActor)
    (if (Components|ComponentHasTag OtherComp "PlayerMeshCapsule")
      (if (not (Variables|Default|GetallTextSeen))
        (Rendering|SetVisibility (Variables|Default|GetWBP_TextBubble) false false)))))

(event EventBeginPlay
  ;[0.15 0.15 0.15 0.5] EBP
  (Variables|Default|SetHasSomethingToSay (not (Utilities|Text|TextIsEmpty (Utilities|Array|Get(acopy) (Variables|Data|GetInteractionTexts)))))
  (bind _aswbp_text_bubble (Utilities|Casting|CastToWBP_TextBubble (UserInterface|GetUserWidgetObject (Variables|Default|GetWBP_TextBubble))))
  (bind _output_get (Variables|Default|SetWBP_TextBubble-Ref _aswbp_text_bubble))
  (if (Variables|Default|GetHasSomethingToSay)
    (bind _reformattedtextlist (CallFunction|Utils-ReformatLineBreaksinTextList (Variables|Data|GetInteractionTexts)))
    (Variables|Data|SetFormattedInteractionTexts _reformattedtextlist)
    (Default|SetText _output_get (Utilities|Array|Get(acopy) (Variables|Data|GetFormattedInteractionTexts)))
    (Variables|Default|SetnextTextIndex 1)))

(event EventOnInteract
  ;[0.15 0.15 0.15 0.5] OnInteract
  (if (and (Variables|Default|GetHasSomethingToSay) (Variables|Default|GetisVisible))
    (if (not (Variables|Default|GetcurrentTextIsLast))
      (if (Variables|Default|GetallTextSeen)
        (Rendering|SetVisibility (Variables|Default|GetWBP_TextBubble) true false)
        (Variables|Default|SetallTextSeen false))
      (Default|SetText (Variables|Default|GetWBP_TextBubble-Ref) (Utilities|Array|Get(acopy) (Variables|Data|GetFormattedInteractionTexts) (Variables|Default|GetnextTextIndex)))
      (Math|Integer|IncrementInt (Variables|Default|GetnextTextIndex)
        (:%20%20
          (if (>= (Variables|Default|GetnextTextIndex) (Utilities|Array|Length (Variables|Data|GetFormattedInteractionTexts))) ; currentTextIsLast
            (Variables|Default|SetcurrentTextIsLast true)
            (Default|ShoworHideInteractionIndicator (Variables|Default|GetWBP_TextBubble-Ref) false)
            (if (not (Variables|Default|GetallTextSeenOnceAtLeast))
              (Variables|Default|SetallTextSeenOnceAtLeast true)))))
      (else
        (Rendering|SetVisibility (Variables|Default|GetWBP_TextBubble) false false)
        (Variables|Default|SetnextTextIndex 0)
        (Variables|Default|SetallTextSeen true)
        (Variables|Default|SetcurrentTextIsLast false)
        (Default|ShoworHideInteractionIndicator (Variables|Default|GetWBP_TextBubble-Ref) true)))))

(fn ConstructionScript
  (Rendering|SetCastShadow (Variables|Default|GetWBP_TextBubble) false))

(fn UnHideTotem
  (Utilities|FlowControl|Sequence
    (:then_0
      (Rendering|SetVisibility (Variables|Default|GetSM_InstructionTotem) true false)
      (Variables|Default|SetisVisible true))
    (:then_1
      ;[0.1812 0.3351 0.1681 0.5] debug parce que ça marche pas, au spawn à l'endroit normal ça l'active quand même
      (if false
        (if (Math|Boolean|ANDBoolean (Variables|Default|GetHasSomethingToSay) (Variables|Default|GetisVisible) (Utilities|Array|IsNotEmpty (Collision|GetOverlappingActors (Variables|Default|GetDetectPlayer-SphereCollision) 0 :!class /Script/Engine.PrimitiveComponent)) (not (Variables|Default|GetallTextSeen)))
          (Rendering|SetVisibility (Variables|Default|GetWBP_TextBubble) true false))))))