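; BP_Case is a tile actor in the Patterns minigame that can be flagged as fake, so that it drops away when the player touches it.
; BeginPlay creates a dynamic instance of M_Case for the mesh.
; When the first-person character overlaps the Box of a FakeCase, a slowed Timeline repeatedly lowers the actor, then destroys it.
; PlayFlash is empty, and the flash timeline and Intensity logic are unwired.
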(event OnComponentBeginOverlap(Box)
  (params (OverlappedComponent :type Primitive%20Component%20Object%20Reference) (OtherActor :type Actor%20Object%20Reference) (OtherComp :type Primitive%20Component%20Object%20Reference) (OtherBodyIndex :type Integer) (bFromSweep :type Boolean) (SweepResult :type Hit%20Result%20Structure%20%28by%20ref%29))
  (bind _returnvalue (Transformation|GetActorLocation))
  (if (Variables|Default|GetFakeCase)
    (Utilities|Casting|CastToBP_FirstPersonCharacter OtherActor)
    (Components|Timeline|SetPlayRate (Variables|Default|GetTimeline) (/ 1.0 1e+01))
    (bind _float (Timeline|Timeline Play)
      (:Update
        (Transformation|SetActorLocation (Math|Vector|MakeVector (.x _returnvalue) (.y _returnvalue) (- (.z _returnvalue) (* _float 1e+02))) false false))
      (:Finished
        (Actor|DestroyActor)))))

(event Custom|PlayFlash)

(event EventBeginPlay
  (bind _returnvalue (Rendering|Material|CreateDynamicMaterialInstance "/Game/_Main/Maps/MiniGame_Patterns/Pattern/M_Case.M_Case" "None" "None" :!class /Script/Engine.KismetMaterialLibrary))
  (Variables|Default|SetDynamicMaterial _returnvalue)
  (Rendering|Material|SetMaterial (Variables|Default|GetStaticMesh) 0 0))

(event Collision|EventActorBeginOverlap
  (params (OtherActor :type Actor%20Object%20Reference)))

(event EventTick
  (params (DeltaSeconds :type Float%20%28single-precision%29)))

(fn ConstructionScript)