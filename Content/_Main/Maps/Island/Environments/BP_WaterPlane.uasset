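; Water plane for the Island map that bobs vertically, carrying floating props with it to imitate waves.
; After a short delay on BeginPlay, it attaches every actor tagged ShouldFloat to itself, keeping world transforms, and stores its own starting height.
; A timeline track then lerps the plane's Z between that height and WaveHeight below it, so attached actors follow through the attachment.
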(event EventBeginPlay
  (Utilities|FlowControl|Delay 3.0)
  (Utilities|FlowControl|Sequence
    (:then_0
      ;[0.15 0.15 0.15 0.5] Met tous les acteurs qui doivent flotter dans un seul array (dont self)
      (bind _outactors (Actor|GetAllActorswithTag "ShouldFloat"))
      (for _array_element _outactors
        (Transformation|AttachActorToActor _array_element self "None" "KeepWorld" "KeepWorld" "KeepWorld" true))
      (Utilities|Array|Add (Variables|Default|GetFloatingActors-Refs) self))
    (:then_1
      (for _array_element_2 (Variables|Default|GetFloatingActors-Refs)
        (Utilities|Array|Add (Variables|Default|GetFloatingActorsPreviousZs) (.z (Transformation|GetActorLocation _array_element_2))))
      (bind _wavefloattrack (Timeline|Timeline_0 Play)
        (:Update
          (for (_array_element_3 _array_index) (Variables|Default|GetFloatingActors-Refs)
            (Transformation|SetActorLocation _array_element_3 (Math|Vector|MakeVector (.x (Transformation|GetActorLocation _array_element_3)) (.y (Transformation|GetActorLocation _array_element_3)) (Math|Float|Lerp (Utilities|Array|Get(acopy) (Variables|Default|GetFloatingActorsPreviousZs) _array_index) (- (Utilities|Array|Get(acopy) (Variables|Default|GetFloatingActorsPreviousZs) _array_index) (Variables|Default|GetWaveHeight)) _wavefloattrack)) false false)))))))

(fn ConstructionScript)