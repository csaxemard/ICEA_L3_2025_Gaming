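; BP_BoardPath is a board path actor that uses a spline to lay out tiles for the island board.
; The construction script and BeginPlay mark spline points with tinted paper sprites.
; Older logic to auto-fit the spline, compute evenly timed tile transforms and spawn TilesToCreate classes into PathTileList is disabled behind constant branches, so only the point markers run.
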(event EventBeginPlay
  (Utilities|FlowControl|Sequence
    (:then_0
      (if (not true)
        ;[0.05032 0.3021 0.03776 0.2] debug
        (if (Variables|Default|GetDebug-Enabled?)
          (bind _returnvalue (Actor|GetActorOfClass "/Game/OldProject/Blueprints/BP_GameMaster.BP_GameMaster_C"))
          (Variables|Ref|SetGameMasterRef _returnvalue)
          ;[0.15 0.15 0.15 0.5] Spawn squares at planned location
          (for (_array_element _array_index) (Variables|Default|GetTilesTransforms)
            (bind _returnvalue_2 (Game|SpawnActorfromClass (Utilities|Array|Get(acopy) (Variables|Data-AutoFitSplinetoNbOfTiles|GetTilesToCreate) _array_index) (Math|Transform|MakeTransform (.location _array_element) (Math|Rotator|MakeRotator 0.0 0.0 (.yaw (.rotation _array_element))) "1.000000,1.000000,1.000000") "AdjustIfPossibleButAlwaysSpawn" "MultiplyWithRoot" 0 0 (.TileColor (Utilities|GetClassDefaults (Utilities|Array|Get(acopy) (Variables|Data-AutoFitSplinetoNbOfTiles|GetTilesToCreate) _array_index))) 0 false 0))
            (Utilities|Array|Add (Variables|Data|GetPathTileList) _returnvalue_2)))))
    (:then_1
      (for _index (range (Spline|GetNumberOfSplinePoints (Variables|Default|GetSpline)) 0)
        (bind _returnvalue_3 (AddComponent|AddPaperSpriteComponent false (Math|Transform|MakeTransform (Spline|GetLocationatSplinePoint (Variables|Default|GetSpline) _index "World") "0, 0, 0" "1.000000,1.000000,1.000000")))
        (Sprite|SetSpriteColor _returnvalue_3 "(R=0.911458,G=0.442184,B=0.069334,A=0.500000)")))))

(fn ConstructionScript
  (bind _spline (Variables|Default|GetSpline))
  (bind _spline_2 (Variables|Default|GetSpline))
  (bind _gamemasterref (Variables|Ref|GetGameMasterRef))
  (bind _tilegap (Variables|/Game/OldProject/Blueprints/BP_GameMaster.BP_GameMaster_C|GetTileGap _gamemasterref))
  (Utilities|FlowControl|Sequence
    (:then_0
      ;[0.1812 0.3351 0.1681 0.5] debug, n'exécute pas old project code
      (if (not true)
        (CallFunction|AutoFitSplinetoNumberOfTiles)
        ;[0.15 0.15 0.15 0.5] Compute possible squares count in that spline
        (Variables|Default|SetPossibleSquareCount (Class|KismetMathLibrary|FFloor64 (/ (+ (Spline|GetSplineLength (Variables|Default|GetSpline)) _tilegap) (+ (.x (Variables|/Game/OldProject/Blueprints/BP_GameMaster.BP_GameMaster_C|GetTileDimensions _gamemasterref)) _tilegap))))
        ;[0.15 0.15 0.15 0.5] Set future squares transforms
        (Variables|/Script/Engine.SplineComponent|SetDuration _spline_2 (Math|Conversions|ToFloat(Integer) (Variables|Default|GetPossibleSquareCount)))
        (for _index (range 1 (Math|Conversions|ToInteger(Byte) (Variables|Default|GetPossibleSquareCount)))
          (bind _returnvalue (Utilities|Array|Add (Variables|Default|GetTilesTransforms) (Spline|GetTransformatTime _spline_2 (- (Math|Conversions|ToFloat(Integer) _index) 1.0) "World" false false)))
          (bind _returnvalue_2 (AddComponent|AddPaperSpriteComponent true (Math|Transform|MakeTransform (- (.Location (Math|Transform|BreakTransform (Spline|GetTransformatTime _spline_2 (- (Math|Conversions|ToFloat(Integer) _index) 1.0) "World" false false))) "15.000000,0.000000,-15.000000") (Math|Rotator|MakeRotator 9e+01 0.0 (.yaw (.Rotation (Math|Transform|BreakTransform (Spline|GetTransformatTime _spline_2 (- (Math|Conversions|ToFloat(Integer) _index) 1.0) "World" false false))))) "0.900000,0.900000,0.900000")))
          (Sprite|SetSpriteColor _returnvalue_2 (.TileColor (Utilities|GetClassDefaults (Utilities|Array|Get(acopy) (Variables|Data-AutoFitSplinetoNbOfTiles|GetTilesToCreate) _returnvalue)))))))
    (:then_1
      (for _index_2 (range 0 (Spline|GetNumberOfSplinePoints (Variables|Default|GetSpline)))
        (bind _returnvalue_3 (AddComponent|AddPaperSpriteComponent true (Math|Transform|MakeTransform (Math|Vector|MakeVector (.x (Spline|GetLocationatSplinePoint _spline _index_2 "World")) (.y (Spline|GetLocationatSplinePoint _spline _index_2 "World")) (+ (.z (Spline|GetLocationatSplinePoint _spline _index_2 "World")) 1e+01)) (Math|Rotator|MakeRotator (+ (.roll (Spline|GetRotationatSplinePoint _spline _index_2 "World")) 9e+01) (.pitch (Spline|GetRotationatSplinePoint _spline _index_2 "World")) (.yaw (Spline|GetRotationatSplinePoint _spline _index_2 "World"))) "0.900000,0.900000,0.900000")))
        (Sprite|SetSpriteColor _returnvalue_3 "(R=0.911458,G=0.911458,B=0.911458,A=1.000000)")))))

(fn AutoFitSplinetoNumberOfTiles
  (bind _returnvalue (Transformation|GetActorLocation))
  (bind _spline (Variables|Default|GetSpline))
  (bind _gamemasterref (Variables|Ref|GetGameMasterRef))
  (if (Variables|Data-AutoFitSplineToNbOfTiles|GetAutoFit?)
    (LocalVariables|SetL-PreviousForwardVector (Math|Vector|GetForwardVector _spline))
    (Spline|ClearSplinePoints _spline true)
    (Spline|AddSplinePoint _spline _returnvalue "World" true)
    (Spline|AddSplinePoint _spline (+ _returnvalue (* (* (+ (.x (Variables|/Game/OldProject/Blueprints/BP_GameMaster.BP_GameMaster_C|GetTileDimensions _gamemasterref)) (Variables|/Game/OldProject/Blueprints/BP_GameMaster.BP_GameMaster_C|GetTileGap _gamemasterref)) (Variables|Data-AutoFitSplineToNbOfTiles|GetNumberOfTiles)) (LocalVariables|GetL-PreviousForwardVector))) "World" true)))