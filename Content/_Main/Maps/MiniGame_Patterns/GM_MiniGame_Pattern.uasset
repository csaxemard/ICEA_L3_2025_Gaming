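; Game mode for the Pattern minigame, where the player crosses a bridge of wooden pallets, some of them fragile.
; On BeginPlay it randomly marks each BP_Case as fake or adds it to TrueCaseList, then binds events on BP_EndDoor and BP_Falling.
; WBP_MsgModal shows intro, success and failure messages.
; Dismissing the intro enables mouse clicks; dismissing success quits the game, while dismissing failure opens the Island level.
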(event Custom|EndMiniGame
  (bind _returnvalue (UserInterface|CreateWidget "/Game/_Main/UI/WBP_MsgModal.WBP_MsgModal_C" 0 "" true true "NewEnumerator1"))
  (Rendering|Components|TextRender|SetText (Variables|/Game/_Main/UI/WBP_MsgModal.WBP_MsgModal_C|Getmessage_umgText _returnvalue) (Utilities|Text|FormatText "Félicitations ! Vous pouvez regagner la partie principale !"))
  (Variables|/Script/Engine.PlayerController|SetbShowMouseCursor (Game|GetPlayerController 0) true)
  (UserInterface|Viewport|AddtoPlayerScreen _returnvalue)
  (EventDispatchers|BindEventtoModalDismissed _returnvalue (delegate Custom|CustomEvent)))

(event Custom|StartMiniGme
  ;[0.15 0.15 0.15 0.5] Comment
  (bind _returnvalue (UserInterface|CreateWidget "/Game/_Main/UI/WBP_MsgModal.WBP_MsgModal_C" 0 "" true true "NewEnumerator1"))
  (Rendering|Components|TextRender|SetText (Variables|/Game/_Main/UI/WBP_MsgModal.WBP_MsgModal_C|Getmessage_umgText _returnvalue) (Utilities|Text|FormatText "Bienvenue ! Durant cette épreuve, vous devrez tarverser un pont compé de palettes de bois mais attention, certaines palettes sont fragiles ! Un faux pas et..."))
  (UserInterface|Viewport|AddtoPlayerScreen _returnvalue)
  (EventDispatchers|BindEventtoModalDismissed _returnvalue (delegate Custom|OnMessageDismissed)))

(event Custom|OnMessageDismissed
  (bind _returnvalue (Game|GetPlayerController 0))
  ;[0.15 0.15 0.15 0.5] Comment
  (Input|SetInputModeGameandUI _returnvalue 0 "DoNotLock" true false)
  (Variables|/Script/Engine.PlayerController|SetbShowMouseCursor _returnvalue true)
  (Variables|/Script/Engine.PlayerController|SetbEnableClickEvents _returnvalue true))

(event Custom|CustomEvent
  (Game|QuitGame 0 "Quit" false))

(event Custom|FailMiniGame
  (bind _returnvalue (UserInterface|CreateWidget "/Game/_Main/UI/WBP_MsgModal.WBP_MsgModal_C" 0 "" true true "NewEnumerator1"))
  (Rendering|Components|TextRender|SetText (Variables|/Game/_Main/UI/WBP_MsgModal.WBP_MsgModal_C|Getmessage_umgText _returnvalue) (Utilities|Text|FormatText "Vous avez faillit à cette épreuve. Vous pouvez regagner l'île principale, mais vous ne gagnez pas de temps bonus."))
  (Variables|/Script/Engine.PlayerController|SetbShowMouseCursor (Game|GetPlayerController 0) true)
  (UserInterface|Viewport|AddtoPlayerScreen _returnvalue)
  (EventDispatchers|BindEventtoModalDismissed _returnvalue (delegate Custom|QuitMiniGame)))

(event Custom|QuitMiniGame
  (Game|OpenLevel(byObjectReference) "/Game/_Main/Maps/Island.Island"))

(event EventTick
  (params (DeltaSeconds :type Float%20%28single-precision%29)))

(event EventBeginPlay
  (Utilities|FlowControl|Sequence
    (:then_0
      (bind _outactors (Actor|GetAllActorsOfClass "/Game/_Main/Maps/MiniGame_Patterns/Pattern/BP_Case.BP_Case_C"))
      (Variables|Default|SetListeCase _outactors)
      (bind _returnvalue (Actor|GetActorOfClass "/Game/_Main/Maps/MiniGame_Patterns/Pattern/BP_EndDoor.BP_EndDoor_C"))
      (Variables|Default|SetEndDoor _returnvalue)
      (bind _returnvalue_2 (Actor|GetActorOfClass "/Game/_Main/Maps/MiniGame_Patterns/Pattern/BP_Falling.BP_Falling_C"))
      (Variables|Default|SetFalling _returnvalue_2))
    (:then_1
      (for _array_element (Variables|Default|GetListeCase)
        (if (== (Math|Random|RandomIntegerinRange 1 2) 1)
          (Variables|/Game/_Main/Maps/MiniGame_Patterns/Pattern/BP_Case.BP_Case_C|SetFakeCase _array_element true)
          (else
            (Utilities|Array|Add (Variables|Default|GetTrueCaseList) _array_element))))
      (EventDispatchers|BindEventtoPlayerPassedDoor (Variables|Default|GetEndDoor) (EventDispatchers|CreateEvent :!event Custom|EndMiniGame))
      (EventDispatchers|BindEventtoPlayerFall (Variables|Default|GetFalling) (EventDispatchers|CreateEvent :!event Custom|FailMiniGame)))
    (:then_2
      (CallFunction|StartMiniGme))))

(fn ConstructionScript)