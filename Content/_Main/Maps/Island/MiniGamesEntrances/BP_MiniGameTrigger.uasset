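; Interactable island actor that serves as an entrance to a mini-game, loading its level when the player interacts with it.
; On BeginPlay it prints an error if no target level is set and styles its widget marker with a star icon.
; A timeline applies vertical world offsets to animate the actor's height.
; Interaction calls the entered-mini-game event, then opens the level from the soft world reference.
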(event EventBeginPlay
  (Utilities|FlowControl|Sequence
    (:then_0
      (if (Utilities|IsValidSoftObjectReference (.worldasset (Variables|Default|GetMiniGameToOpen)))
        _
        (else
          (Development|PrintText (Utilities|Text|FormatText "({name}) Erreur : Pas de niveau à ouvrir défini" (Utilities|GetDisplayName self)) true true "(R=0.376736,G=0.054287,B=0.054287,A=1.000000)" 1e+01)))
      (bind _aswbp_actor_marker (Utilities|Casting|CastToWBP_ActorMarker (UserInterface|GetUserWidgetObject (Variables|Default|GetWBP_Marker))))
      (Variables|Default|SetWBP%20Actor%20Marker-Ref _aswbp_actor_marker)
      (Default|SetIconandColor _aswbp_actor_marker "/Game/_Main/Maps/Island/OverviewCam/T_Star_MarkerIcon.T_Star_MarkerIcon" 4))
    (:then_1
      (bind _float (Timeline|Timeline Play)
        (:Update
          (Transformation|AddActorWorldOffset (Math|Vector|MakeVector 0.0 0.0 (Math|Float|Lerp -1.0 1.0 _float))))))))

(event EventOnInteract
  (Default|CallEnteredMiniGame)
  (Game|OpenLevel(byObjectReference) (Utilities|Struct|BreakSoftWorldReference (Variables|Default|GetMiniGameToOpen))))

(fn ConstructionScript)