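; Game mode for the totem mini-game, an intelligence challenge asking the player to solve a random addition.
; On BeginPlay it removes debug-disabled actors, stores the sum as NumberToFind, has BP_TotemSpawner generate totems and binds each one's correct-totem event.
; It then sets Game and UI input and shows the question in a modal.
; The end event shows a win message; its dismissal only prints, as quitting is disabled.
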(event Custom|onModalDismissed
  ;[0.15 0.15 0.15 0.5] endMiniGame
  (Development|PrintString "Mini Game finished")
  (Game|QuitGame 0 "Quit" false))

(event Custom|endMiniGame
  ;[0.15 0.15 0.15 0.5] endMiniGame
  (bind _wbp_minigamemsg_ref (CallFunction|UIShowMessage "Gagné ! 
Avancez de 2 cases " true true "NewEnumerator0"))
  (EventDispatchers|BindEventtoModalDismissed _wbp_minigamemsg_ref (delegate Custom|onModalDismissed)))

(event Custom|startMiniGame
  ;[0.15 0.15 0.15 0.5] startMiniGame
  (CallFunction|UIShowMessage (Utilities|Text|FormatText "L'île vous met au défi - Epreuve d'intelligence 
 
Il est écrit : 
\"Seuls les plus intelligents auront la vie sauve.\" 
\"Combien font {nombre1} + {nombre2} ?\"" (Variables|GameplayLogic|GetequationNumber1) (Variables|GameplayLogic|GetequationNumber2)) true true "NewEnumerator0"))

(event EventBeginPlay
  ;[0.15 0.15 0.15 0.5] EBP : Init MiniGame
  (Utilities|FlowControl|Sequence
    (:then_0
      ;;[0.1812 0.3351 0.1681 0.5] Définit manuellement variables editables
      (Variables|Editables|SetnumberOfTotemsToSpawn 10)
      (Variables|Editables|SetminEquationNumber 1)
      (Variables|Editables|SetmaxEquationNumber 10)
      ;;[0.1812 0.3351 0.1681 0.5] debug : disabled actors
      (bind _outactors (Actor|GetAllActorswithTag "debug-disabled"))
      (for _array_element _outactors
        (Actor|DestroyActor _array_element)))
    (:then_1
      (|initCurrentActorsRefs)
      ;;[0.15 0.15 0.15 0.5] Init logique gameplay pour le mini jeu
      ;; Définit le nombre à trouver
      (bind _output_get (Variables|GameplayLogic|SetequationNumber1 (Math|Random|RandomIntegerinRange (Variables|Editables|GetminEquationNumber) (Variables|Editables|GetmaxEquationNumber))))
      (bind _output_get_2 (Variables|GameplayLogic|SetequationNumber2 (Math|Random|RandomIntegerinRange (Variables|Editables|GetminEquationNumber) (Variables|Editables|GetmaxEquationNumber))))
      (Variables|GameplayLogic|SetnumberToFind (+ _output_get _output_get_2))
      ;;[0.15 0.15 0.15 0.5] Génère actors pour le mini jeu
      (bind (_totemsactorslist _correcttotemsactorslist) (Default|GenerateTotems (Variables|ActorsRefs|GettotemSpawnerActor) (Variables|Editables|GetnumberOfTotemsToSpawn)))
      (Variables|ActorsRefs|SettotemsActorsList _totemsactorslist)
      (Variables|ActorsRefs|SetcorrectTotemsActorsList _correcttotemsactorslist))
    (:then_2
      ;;[0.15 0.15 0.15 0.5] initHandlers_toEndMiniGame
      (if (Utilities|Array|IsNotEmpty (Variables|ActorsRefs|GettotemsActorsList))
        (for _array_element_2 (Variables|ActorsRefs|GettotemsActorsList)
          (EventDispatchers|BindEventtoCorrectTotemFound _array_element_2 (EventDispatchers|CreateEvent :!event Custom|endMiniGame)))
        (else
          (Development|PrintString "[GM_MiniGame1 - Init] Erreur : correctTotemsActorsList is empty"))))
    (:then_3
      ;;[0.15 0.15 0.15 0.5] Set up mouvements joueur pour le mini jeu
      (CallFunction|SetInputGameandUI)
      (CallFunction|StartMiniGame))))

(fn ConstructionScript)

(fn SetInputGameandUI
  (bind _returnvalue (Game|GetPlayerController 0))
  (Input|SetInputModeGameandUI _returnvalue 0 "DoNotLock" true false)
  (Variables|/Script/Engine.PlayerController|SetbShowMouseCursor _returnvalue true)
  (Variables|/Script/Engine.PlayerController|SetbEnableClickEvents _returnvalue true))