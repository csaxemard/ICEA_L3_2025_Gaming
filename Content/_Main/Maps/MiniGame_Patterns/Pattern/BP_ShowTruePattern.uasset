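; Actor for the pattern mini-game that briefly shows the true pattern when its ButtonShow is clicked.
; It gets the TrueCaseList from GM_MiniGame_Pattern and sets each case's Cube material to M_Case.
; After a short delay it switches those cubes to MI_vigjfivg.
; A DoOnce with no reset wired limits the reveal to a single use.
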(event OnClicked(ButtonShow)
  (params (TouchedComponent :type Primitive%20Component%20Object%20Reference) (ButtonPressed :type Key%20Structure))
  (Utilities|FlowControl|DoOnce false
    (:Completed
      (bind _asgm_mini_game_pattern (Utilities|Casting|CastToGM_MiniGame_Pattern (Game|GetGameMode)))
      (for _array_element (Variables|/Game/_Main/Maps/MiniGame_Patterns/GM_MiniGame_Pattern.GM_MiniGame_Pattern_C|GetTrueCaseList _asgm_mini_game_pattern)
        (Rendering|Material|SetMaterial (Variables|/Game/_Main/Maps/MiniGame_Patterns/Pattern/BP_Case.BP_Case_C|GetCube _array_element) 0 "/Game/_Main/Maps/MiniGame_Patterns/Pattern/M_Case.M_Case"))
      (Utilities|FlowControl|Delay 2.0)
      (for _array_element_2 (Variables|/Game/_Main/Maps/MiniGame_Patterns/GM_MiniGame_Pattern.GM_MiniGame_Pattern_C|GetTrueCaseList _asgm_mini_game_pattern)
        (Rendering|Material|SetMaterial (Variables|/Game/_Main/Maps/MiniGame_Patterns/Pattern/BP_Case.BP_Case_C|GetCube _array_element_2) 0 "/Game/Fab/Megascans/Surfaces/Old_Plywood_vigjfivg/Low/MI_vigjfivg.MI_vigjfivg")))))

(event Collision|EventActorBeginOverlap
  (params (OtherActor :type Actor%20Object%20Reference)))

(event EventTick
  (params (DeltaSeconds :type Float%20%28single-precision%29)))

(fn ConstructionScript)