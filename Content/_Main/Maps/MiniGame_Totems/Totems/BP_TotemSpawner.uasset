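; BP_TotemSpawner spawns the numbered totems for a number-finding minigame and returns lists of all totems and the correct ones.
; GenerateTotems reads the target number from GM_MiniGame_1, forces the first totem to match, and randomizes the rest within twice the equation range.
; Totems spawn at fixed height with random yaw, using GetRandomLocationInSpawnArea for X/Y.
; That function's box-based random position math appears unconnected.
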(event EventBeginPlay)

(event Collision|EventActorBeginOverlap
  (params (OtherActor :type Actor%20Object%20Reference)))

(event EventTick
  (params (DeltaSeconds :type Float%20%28single-precision%29)))

(fn ConstructionScript)

(fn GenerateTotems
  (params (numberOfTotemsToSpawn :type Integer))
  (bind (_x _y) (|getRandomLocationInSpawnArea))
  (Utilities|FlowControl|Sequence
    (:then_0
      (bind _asgm_mini_game_1 (Utilities|Casting|CastToGM_MiniGame_1 (Game|GetGameMode)))
      (bind _output_get (LocalVariables|SetL-GameModeRef _asgm_mini_game_1))
      (LocalVariables|SetL-numberToFind (Variables|/Game/_Main/Maps/MiniGame_Totems/GM_MiniGame_1.GM_MiniGame_1_C|GetnumberToFind _output_get)))
    (:then_1
      (for _index (range 1 numberOfTotemsToSpawn)
        (LocalVariables|SetL-generatedTotemId _index)
        (if (== _index 1)
          ;[0.15 0.15 0.15 0.5] Force au moins un totem correct
          (LocalVariables|SetL-generatedTotemNumber (LocalVariables|GetL-numberToFind))
          (else
            (LocalVariables|SetL-generatedTotemNumber (Math|Random|RandomIntegerinRange (* (Variables|/Game/_Main/Maps/MiniGame_Totems/GM_MiniGame_1.GM_MiniGame_1_C|GetminEquationNumber (LocalVariables|GetL-GameModeRef)) 2) (* (Variables|/Game/_Main/Maps/MiniGame_Totems/GM_MiniGame_1.GM_MiniGame_1_C|GetmaxEquationNumber (LocalVariables|GetL-GameModeRef)) 2)))))
        (LocalVariables|SetL-isGeneratedTotemCorrect (== (LocalVariables|GetL-generatedTotemNumber) (LocalVariables|GetL-numberToFind)))
        (bind _returnvalue (Game|SpawnActorfromClass "/Game/_Main/Maps/MiniGame_Totems/Totems/BP_Totem.BP_Totem_C" (Math|Transform|MakeTransform (Math|Vector|MakeVector _x _y 5e+01) (Math|Rotator|MakeRotator 0.0 0.0 (.yaw (Math|Random|RandomRotator false)))) "AdjustIfPossibleButAlwaysSpawn" "MultiplyWithRoot" 0 (LocalVariables|GetL-generatedTotemId) (LocalVariables|GetL-generatedTotemNumber) (LocalVariables|GetL-isGeneratedTotemCorrect) 0))
        (Utilities|Array|Add (LocalVariables|GetL-totemsActorsList) _returnvalue)
        (if (LocalVariables|GetL-isGeneratedTotemCorrect)
          (Utilities|Array|Add (LocalVariables|GetL-correctTotemsActorsList) _returnvalue))))
    (:then_2
      (return (LocalVariables|GetL-totemsActorsList) (LocalVariables|GetL-correctTotemsActorsList)))))