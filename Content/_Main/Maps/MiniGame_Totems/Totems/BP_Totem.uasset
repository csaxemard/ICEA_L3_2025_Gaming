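; Clickable, numbered totem actor for the Totems minigame.
; The construction script picks one of four totem meshes at random, with matching material and scale, and BeginPlay writes TotemNumber into its widget component.
; Clicking the mesh calls CorrectTotemFound when the totem is correct, otherwise prints a loss message.
; A debug override currently marks every clicked totem as correct, so the loss branch never runs.
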(event OnClicked(TotemStaticMesh)
  (params (TouchedComponent :type Primitive%20Component%20Object%20Reference) (ButtonPressed :type Key%20Structure))
  ;[0.1812 0.3351 0.1681 0.5] debug
  (Development|PrintString "[BP_Totem - on clicked] Debug : every Totem is correct")
  (Variables|Default|SetisACorrectTotem true)
  (if (Variables|Default|GetisACorrectTotem)
    (Default|CallCorrectTotemFound)
    (else
      (Development|PrintString "Perdu"))))

(event EventBeginPlay
  (Rendering|Components|TextRender|SetText (Variables|/Game/_Main/Maps/MiniGame_Totems/Totems/TotemAssets/WBP_TotemNumber.WBP_TotemNumber_C|GettotemNumber_umgText (.AsWBP%20Totem%20Number (Utilities|Casting|CastToWBP_TotemNumber (UserInterface|GetUserWidgetObject (Variables|Default|GettotemNumberWidget))))) (Utilities|Text|ToText(Integer) (Variables|Default|GettotemNumber))))

(fn ConstructionScript
  (Rendering|SetCastShadow (Variables|Default|GettotemNumberWidget) false)
  (|RandomizeTotemMesh))