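; BP_EndTile is an end tile for the island board, built on a Cube component and labeled with a tile ID.
; It reports its world-space size from the Cube's local bounds multiplied by world scale.
; Setting the ID stores it and writes it to the text of a referenced ID widget.
; SetTileColor and the construction script are empty, so the tile ignores color requests.
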(fn ConstructionScript)

(fn GetTileScaledDimensions
  (bind _cube (Variables|Default|GetCube))
  (bind (_min _max) (Components|StaticMesh|GetLocalBounds _cube))
  (return (* (Transformation|GetWorldScale _cube) (+ (Math|Vector|VectorGetAbs _min) _max))))

(fn SetTileColor
  (params (TileColor :type Linear%20Color%20Structure)))

(fn SetTileIdandUpdateWidget
  (params (TileId :type Integer))
  (bind _output_get (Variables|Data|SetTileId TileId))
  (Variables|/Script/UMG.TextBlock|SetText (Variables|/Game/_Main/Maps/Island/Board/WBP_TileId.WBP_TileId_C|GetTileId (Variables|Default|GetWBP_TileId-Ref)) (Utilities|Text|ToText(Integer) _output_get)))